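; Inventory item for slot index 1 that is meant to give the using character a temporary walk speed boost.
; UseItem rejects use while already boosting, otherwise raises MaxWalkSpeed and starts a timer, with ResetSpeed holding the logic to restore speed and clear the flag.
; As written, MovementRef is set to None instead of the cast character's movement component, and the timer's event shows no link to ResetSpeed.
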(event Custom|ResetSpeed
  (Variables|/Script/Engine.CharacterMovementComponent|SetMaxWalkSpeed (Variables|Default|GetMovementRef) 6e+02)
  (Variables|Default|SetbIsBoosting false))

(fn UseItem
  (params (CharacterRef :type Actor%20Object%20Reference))
  (if (Variables|Default|GetbIsBoosting)
    (return false)
    (else
      (bind _ascharacter (Utilities|Casting|CastToCharacter CharacterRef))
      (Variables|Default|SetbIsBoosting true)
      (bind _output_get (Variables|Default|SetMovementRef 0))
      (Variables|/Script/Engine.CharacterMovementComponent|SetMaxWalkSpeed _output_get 1.2e+03)
      (Utilities|Time|SetTimerbyEvent (EventDispatchers|CreateEvent :!event Custom|ResetSpeed) 5.0)
      (return true))))

(fn GetSlotIndex
  (return 1))