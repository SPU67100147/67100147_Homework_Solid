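; BPC_Inventory is an inventory component that stores one item object per item class, each carrying a quantity.
; AddItem constructs new items at quantity 1, but resets an existing item's quantity to 0 because the increment node is left unconnected.
; UseItem sends a consume message with the user and decrements positive quantities.
; GetItemCount returns the stored quantity, or zero for missing items.
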(event EventBeginPlay)

(event EventTick
  (params (DeltaSeconds :type Float%20%28single-precision%29)))

(fn AddItem
  (params (ItemClass :type BP%20Inventory%20Item%20Base%20Class%20Reference))
  (bind _inventory (Variables|Default|GetInventory))
  (bind (_value _returnvalue) (Utilities|Map|Find _inventory ItemClass))
  (if _returnvalue
    (Variables|/Game/Blueprints/Inventory/BP_InventoryItem_Base.BP_InventoryItem_Base_C|SetQuantity _value 0)
    (else
      (bind _returnvalue_2 (Game|ConstructObjectfromClass self ItemClass))
      (Variables|/Game/Blueprints/Inventory/BP_InventoryItem_Base.BP_InventoryItem_Base_C|SetQuantity _returnvalue_2 1)
      (Utilities|Map|Add (Variables|Default|GetInventory) ItemClass _returnvalue_2))))

(fn UseItem
  (params (ItemClass :type BP%20Inventory%20Item%20Base%20Class%20Reference) (User :type BP%20Player%20Character%20Object%20Reference))
  (bind _inventory (Variables|Default|GetInventory))
  (bind (_value _returnvalue) (Utilities|Map|Find _inventory ItemClass))
  (if _returnvalue
    (if (> (Variables|/Game/Blueprints/Inventory/BP_InventoryItem_Base.BP_InventoryItem_Base_C|GetQuantity _value) 0)
      (Class|BPIConsumeItemable|ConsumeItem(Message) _value User)
      (Variables|/Game/Blueprints/Inventory/BP_InventoryItem_Base.BP_InventoryItem_Base_C|SetQuantity _value (- (Variables|/Game/Blueprints/Inventory/BP_InventoryItem_Base.BP_InventoryItem_Base_C|GetQuantity _value) 1)))))

(fn GetItemCount
  (params (ItemClass :type BP%20Inventory%20Item%20Base%20Class%20Reference))
  (bind _inventory (Variables|Default|GetInventory))
  (bind (_value _returnvalue) (Utilities|Map|Find _inventory ItemClass))
  (if _returnvalue
    (return (Variables|/Game/Blueprints/Inventory/BP_InventoryItem_Base.BP_InventoryItem_Base_C|GetQuantity _value))
    (else
      (return 0))))